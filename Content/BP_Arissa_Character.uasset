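; BP_Arissa_Character is the player character, with Enhanced Input movement and look, health, and respawning.
; BeginPlay registers the input mapping, stores the starting transform as the spawn point, runs Spawning and adds the Arissa HUD widget.
; AnyDamage lowers clamped health; at zero, Spawning refills it and moves the character back to the spawn point.
; A capsule hit against one looked-up actor opens Game_level.
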(event `self.ReceiveBeginPlay`
  (bind _returnvalue (pcsubsystem `EnhancedInputLocalPlayerSubsystem` (`GameplayStatics.GetPlayerController` 0)))
  (`/Engine/EditorBlueprintResources/StandardMacros.IsValid` _returnvalue ; check si input fonctionne ou non
    (:`Is Valid`
      (`EnhancedInputSubsystemInterface.AddMappingContext` _returnvalue "/Game/PlayerInput/PlayerInput_IMC.PlayerInput_IMC" 0 (struct))
      (set `self.CurrentSpawnPoint` (`self.GetTransform`))
      (`self.Spawning`)
      (bind _returnvalue_2 (`|CreateWidget` "/Game/Arissa_Widget_BP.Arissa_Widget_BP_C"))
      (`UserWidget.AddToViewport` _returnvalue_2 0))))

(event `EnhancedInput|/Game/PlayerInput/PlayerMovement_InputAction`
  (params (ActionValue :type "Vector2D Structure") (ElapsedSeconds :type "Float (double-precision)") (TriggeredSeconds :type "Float (double-precision)") (InputAction :type "InputAction Object Reference" :default "/Game/PlayerInput/PlayerMovement_InputAction.PlayerMovement_InputAction"))
  (bind (_returnvalue_roll _returnvalue_pitch _returnvalue_yaw) (`KismetMathLibrary.BreakRotator` (`self.GetControlRotation`)))
  (bind (_returnvalue_roll_2 _returnvalue_pitch_2 _returnvalue_yaw_2) (`KismetMathLibrary.BreakRotator` (`self.GetControlRotation`)))
  (:`Triggered`
    (`self.AddMovementInput` (`KismetMathLibrary.GetRightVector` (`KismetMathLibrary.MakeRotator` _returnvalue_roll 0.0 _returnvalue_yaw)) ActionValue_X) ; for pawn and character
    (`self.AddMovementInput` (`KismetMathLibrary.GetForwardVector` (`KismetMathLibrary.MakeRotator` 0.0 0.0 _returnvalue_yaw_2)) ActionValue_Y)))

(event `self.CapsuleComponent.OnComponentHit`
  (params (HitComponent :type "PrimitiveComponent Object Reference") (OtherActor :type "Actor Object Reference") (OtherComp :type "PrimitiveComponent Object Reference") (NormalImpulse :type "Vector Structure") (Hit :type "HitResult Structure (by ref)"))
  (bind _returnvalue (`GameplayStatics.GetActorOfClass` null))
  (if (== _returnvalue OtherActor)
    (`GameplayStatics.OpenLevel` "Game_level")))

(event `self.ReceiveAnyDamage`
  (params (Damage :type "Float (single-precision)") (DamageType :type "DamageType Object Reference") (InstigatedBy :type "Controller Object Reference") (DamageCauser :type "Actor Object Reference"))
  (bind _output_get (set `self.CurrentHealth` (`KismetMathLibrary.FClamp` (- (`self.CurrentHealth`) Damage) 0.0 (`self.TotalHealth`))))
  (if (== _output_get 0.0)
    (`self.Spawning`)))

(event `EnhancedInput|/Game/PlayerInput/PlayerLook_Action`
  (params (ActionValue :type "Vector2D Structure") (ElapsedSeconds :type "Float (double-precision)") (TriggeredSeconds :type "Float (double-precision)") (InputAction :type "InputAction Object Reference" :default "/Game/PlayerInput/PlayerLook_Action.PlayerLook_Action"))
  (:`Triggered`
    (`self.AddControllerYawInput` ActionValue_X)
    (`self.AddControllerPitchInput` (* ActionValue_Y -1.0))))

(fn `Spawning`
  (set `self.CurrentHealth` (`self.TotalHealth`))
  (`self.K2_SetActorTransform` (`self.CurrentSpawnPoint`)))

(fn `UserConstructionScript`)